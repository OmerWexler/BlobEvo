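; Host-side game manager that runs the repeating round loop of a blob survival game with donuts.
; On game ready it spawns each player's blobs, then loops timed rounds: begin, spawn donuts, wait, end, assess.
; Assessment destroys blobs that should not live and spawns offspring for survivors, rebuilding each player's array.
; Blob and donut spawns and round changes are reported through GameManagerComm, with blob IDs built from player ID and array index.
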(event `Game Ready`
  (`self.SpawnBlobs`)
  (`KismetSystemLibrary.Delay` (`self.TimeBetweenRounds`) :!label _label)
  (`self.BeginRound`)
  (`self.SpawnDonuts`)
  (`KismetSystemLibrary.Delay` (`self.RoundLength`))
  (`self.EndRound`)
  (`self.AssessBlobs`)
  (goto _label))

(event `self.ReceiveBeginPlay`
  (`parent.ReceiveBeginPlay`))

(fn `AssessBlobs`
  (locals (NewBlobsArray :type "Array of /Game/Blueprints/Blob/BlobNPC_BP Object Reference"))
  (bind _newblobsarray (`local.NewBlobsArray`))
  (for _array_element (`self.Players`)
    (set `local.NewBlobsArray` (`|MakeArray`))
    (for _array_element_2 (`PlayerPawn.Blobs` _array_element)
      (bind _asblob_npc_bp (cast `/Game/Blueprints/Blob/BlobNPC_BP` _array_element_2))
      (bind _returnvalue (`Blob.ShouldLive` _asblob_npc_bp))
      (if _returnvalue
        (bind _returnvalue_2 (`Blob.GetNumberOfNewBlobs` _asblob_npc_bp))
        (`KismetArrayLibrary.Array_Add` _newblobsarray _asblob_npc_bp)
        (bind _returnvalue_3 (`Spawner.SpawnByCount` (`self.BlobSpawner`) _returnvalue_2 "/Game/Blueprints/Blob/HostBlobNPC_BP.HostBlobNPC_BP_C"))
        (for _array_element_3 _returnvalue_3
          (bind _ashost_blob_npc_bp (cast `/Game/Blueprints/Blob/HostBlobNPC_BP` _array_element_3))
          (`self.RegisterBlob` _newblobsarray _ashost_blob_npc_bp _array_element))
        (else
          (`self.K2_DestroyActor` _asblob_npc_bp))))
    (set `PlayerPawn.Blobs` (`local.NewBlobsArray`) _array_element)))

(fn `BeginRound`
  (`GameManagerCommunicator.ReportBeginRound` (`self.GameManagerComm`))
  (`parent.BeginRound`))

(fn `EndRound`
  (`GameManagerCommunicator.ReportRoundEnd` (`self.GameManagerComm`))
  (`parent.EndRound`))

(fn `GetBlobClass`
  (returns (BlobClass :type "Blob Class Reference"))
  (return null))

(fn `RegisterBlob`
  (params (TargetArray :type "Array of Blob Object Reference") (Blob :type "/Game/Blueprints/Blob/HostBlobNPC_BP Object Reference") (Player :type "/Game/Blueprints/PlayerPawn/PlayerPawn_BP Object Reference"))
  (bind _id (`/Game/Blueprints/PlayerPawn/PlayerPawn_BP.ID` Player))
  (bind _returnvalue (`KismetArrayLibrary.Array_Add` TargetArray Blob))
  (bind _output_get (set `/Game/Blueprints/Blob/BlobNPC_BP.ID` (`KismetStringLibrary.Concat_StrStr` (`KismetStringLibrary.Conv_IntToString` _id) (`KismetStringLibrary.Conv_IntToString` _returnvalue)) Blob))
  (`GameManagerCommunicator.ReportBlobSpawn` (`self.GameManagerComm`) _output_get _id (`Blob.InitialLocation` Blob)))

(fn `SpawnBlobs`
  (for _array_element (`self.Players`)
    (bind _returnvalue (`Spawner.SpawnByCount` (`self.BlobSpawner`) (`self.NumberOfBlobsPerPlayer`) "/Game/Blueprints/Blob/HostBlobNPC_BP.HostBlobNPC_BP_C"))
    (for _array_element_2 _returnvalue
      (bind _ashost_blob_npc_bp (cast `/Game/Blueprints/Blob/HostBlobNPC_BP` _array_element_2))
      (`self.RegisterBlob` (`PlayerPawn.Blobs` _array_element) _ashost_blob_npc_bp _array_element))))

(fn `SpawnDonuts`
  (bind _returnvalue (`Spawner.SpawnByCount` (`self.DonutSpawner`) (`self.NumberOfDonutsPerRound`) "/Game/Blueprints/Donut_BP.Donut_BP_C"))
  (bind _output_get (set `self.AllDonuts` _returnvalue))
  (for _array_element _output_get
    (bind _asdonut_bp (cast `/Game/Blueprints/Donut_BP` _array_element))
    (`GameManagerCommunicator.ReportDonutSpawn` (`self.GameManagerComm`) (`SceneComponent.K2_GetComponentLocation` (`/Game/Blueprints/Donut_BP.StaticMesh` _asdonut_bp)))))

(fn `SyncBlobsToServer`
  (`GameplayStatics.GetActorOfClass` null))

(fn `UserConstructionScript`)