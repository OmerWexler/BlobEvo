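; Multiplayer game manager that registers the local player with a server and mirrors other players as puppet pawns.
; On BeginPlay it connects and joins through PlayerServerCommunicator, derives the local pawn's ID from the join result, and spawns puppets for earlier players.
; Each tick it polls for newcomers, spawning at most one puppet at the PlayerStart and popping that player from the communicator.
; The Players array tracks all pawns and supplies newcomer IDs from its length.
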(event `self.ReceiveTick`
  (params (DeltaSeconds :type "Float (single-precision)"))
  (`self.ManageNewPlayers`))

(event `self.ReceiveBeginPlay`
  (bind _returnvalue (`GameplayStatics.GetActorOfClass` "/Script/BlobEvo.PlayerServerCommunicator"))
  (set `self.PlayerServerComm` _returnvalue)
  (`self.SetupPlayers`))

(fn `GetBlobClass`
  (returns (BlobClass :type "Blob Class Reference"))
  (return "/Script/BlobEvo.Blob"))

(fn `ManageNewPlayers`
  (bind _players (`self.Players`))
  (bind _returnvalue (`PlayerServerCommunicator.GetNewPlayerCount` (`self.PlayerServerComm`)))
  (`/Engine/EditorBlueprintResources/StandardMacros.CompareInt` _returnvalue
    (:`>`
      (bind _returnvalue_2 (`GameplayStatics.GetActorOfClass` "/Script/Engine.PlayerStart"))
      (bind _returnvalue_3 (`|SpawnActorFromClass` "/Game/Blueprints/PlayerPawn/PlayerPawnPuppet_BP.PlayerPawnPuppet_BP_C" (`KismetMathLibrary.Conv_VectorToTransform` (`self.K2_GetActorLocation` _returnvalue_2)) "AlwaysSpawn" "OverrideRootScale" null null))
      (set `/Game/Blueprints/PlayerPawn/PlayerPawn_BP.ID` (- (`KismetArrayLibrary.Array_Length` _players) 0) _returnvalue_3)
      (`KismetArrayLibrary.Array_Add` _players _returnvalue_3)
      (`PlayerServerCommunicator.PopPlayer` (`self.PlayerServerComm`)))))

(fn `SetupPlayers`
  (bind _playerservercomm (`self.PlayerServerComm`))
  (`ServerCommunicator.Connect` _playerservercomm)
  (bind _outplayercount (`PlayerServerCommunicator.JoinGame` _playerservercomm))
  (bind _returnvalue (`GameplayStatics.GetActorOfClass` "/Game/Blueprints/PlayerPawn/PlayerPawn_BP.PlayerPawn_BP_C"))
  (set `/Game/Blueprints/PlayerPawn/PlayerPawn_BP.ID` (- _outplayercount 1) _returnvalue)
  (`KismetArrayLibrary.Array_Add` (`self.Players`) _returnvalue)
  (bind _returnvalue_2 (`GameplayStatics.GetActorOfClass` "/Script/Engine.PlayerStart"))
  (for _index (range (+ (- _outplayercount 2) 1))
    (bind _returnvalue_3 (`|SpawnActorFromClass` "/Game/Blueprints/PlayerPawn/PlayerPawnPuppet_BP.PlayerPawnPuppet_BP_C" (`KismetMathLibrary.Conv_VectorToTransform` (`self.K2_GetActorLocation` _returnvalue_2)) "AlwaysSpawn" "OverrideRootScale" null null))
    (set `/Game/Blueprints/PlayerPawn/PlayerPawn_BP.ID` _index _returnvalue_3)
    (`KismetArrayLibrary.Array_Add` (`self.Players`) _returnvalue_3)))

(fn `UserConstructionScript`)