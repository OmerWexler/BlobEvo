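; Client-side game manager that mirrors round flow and donut and blob spawns received through GameManagerComm.
; Each Tick it polls that comm object to begin or end rounds and to spawn donuts or client blob NPCs at received locations.
; Spawned blobs take the received ID and join the owning player's Blobs array.
; At round end it destroys blobs failing ShouldLive and rebuilds each player's array before running the parent EndRound.
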(event `self.ReceiveBeginPlay`
  (`parent.ReceiveBeginPlay`))

(event `self.ReceiveTick`
  (params (DeltaSeconds :type "Float (single-precision)"))
  (`parent.ReceiveTick` DeltaSeconds)
  (bind _returnvalue (`GameManagerCommunicator.CheckIfRoundBegan` (`self.GameManagerComm`)))
  (if _returnvalue
    (`self.BeginRound`))
  (bind _returnvalue_2 (`GameManagerCommunicator.CheckIfRoundEnded` (`self.GameManagerComm`)))
  (if _returnvalue_2
    (`self.EndRound`))
  (bind (_spawnlocation _returnvalue_3) (`GameManagerCommunicator.ReceiveDonutSpawn` (`self.GameManagerComm`)))
  (if _returnvalue_3
    (`self.SpawnDonut` _spawnlocation))
  (bind (_blobid _playerid _spawnlocation_2 _returnvalue_4) (`GameManagerCommunicator.ReceiveBlobSpawn` (`self.GameManagerComm`)))
  (if _returnvalue_4
    (`self.SpawnBlob` _spawnlocation_2 _blobid _playerid)))

(fn `AssesBlobs`
  (locals (NewBlobsArray :type "Array of Blob Object Reference"))
  (`GameplayStatics.GetActorOfClass` "/Game/Blueprints/Spawners/BlobSpawner_BP.BlobSpawner_BP_C")
  (for _array_element (`self.Players`)
    (set `local.NewBlobsArray` (`|MakeArray`))
    (for _array_element_2 (`PlayerPawn.Blobs` _array_element)
      (bind _asblob_npc_bp (cast `/Game/Blueprints/Blob/BlobNPC_BP` _array_element_2))
      (bind _returnvalue (`Blob.ShouldLive` _asblob_npc_bp))
      (if _returnvalue
        (`KismetArrayLibrary.Array_Add` (`local.NewBlobsArray`) _asblob_npc_bp)
        (else
          (`self.K2_DestroyActor` _asblob_npc_bp))))
    (set `PlayerPawn.Blobs` (`local.NewBlobsArray`) _array_element)))

(fn `EndRound`
  (`self.AssesBlobs`)
  (`parent.EndRound`))

(fn `SpawnBlob`
  (params (SpawnLocation :type "Vector Structure") (BlobID :type String) (PlayerID :type Integer))
  (bind _returnvalue (`Spawner.SpawnByLocation` (`self.BlobSpawner`) SpawnLocation "/Game/Blueprints/Blob/ClientBlobNPC_BP.ClientBlobNPC_BP_C"))
  (bind _asblob_npc_bp (cast `/Game/Blueprints/Blob/BlobNPC_BP` _returnvalue))
  (set `/Game/Blueprints/Blob/BlobNPC_BP.ID` BlobID _asblob_npc_bp)
  (`KismetArrayLibrary.Array_Add` (`PlayerPawn.Blobs` (`|GetArrayItem` (`self.Players`) PlayerID)) _asblob_npc_bp))

(fn `SpawnDonut`
  (params (`SpawnLocation ` :type "Vector Structure"))
  (`Spawner.SpawnByLocation` (`self.DonutSpawner`) `SpawnLocation ` "/Game/Blueprints/Donut_BP.Donut_BP_C"))

(fn `UserConstructionScript`)