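; NPC blob that wanders the map during a round, eating any donut it hits.
; Tick drives the physics mesh at constant speed along its negative Y axis with a fixed downward velocity, picking a random yaw at random intervals.
; Hitting a Spawner turns it toward the world origin and restarts that timer.
; Round start also faces it to center and clears its donut count; round end stops it and restores its initial location.
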(event `self.ReceiveHit`
  (params (MyComp :type "PrimitiveComponent Object Reference") (Other :type "Actor Object Reference") (OtherComp :type "PrimitiveComponent Object Reference") (bSelfMoved :type Boolean) (HitLocation :type "Vector Structure") (HitNormal :type "Vector Structure") (NormalImpulse :type "Vector Structure") (Hit :type "HitResult Structure (by ref)"))
  (bind _asdonut_bp (cast `/Game/Blueprints/Donut_BP` Other)
    (:`then`
      (`self.EatDonut` _asdonut_bp))
    (:`CastFailed`
      (cast `Spawner` Other)
      (set `self.bHitSpawner` true)
      (`self.LookAtCenterOfMap`))))

(event `self.ReceiveTick`
  (params (DeltaSeconds :type "Float (single-precision)"))
  (`self.KeepVelocity` DeltaSeconds))

(event `BeginRound`
  (`self.RandomizeTimeToRedirection`)
  (`self.LookAtCenterOfMap`)
  (set `self.bIsInRound` true)
  (set `self.DonutsEaten` 0))

(event `EndRound`
  (set `self.bIsInRound` false)
  (`PrimitiveComponent.SetPhysicsLinearVelocity` (`self.StaticMesh`) (0.0 0.0 0.0) false "None")
  (`SceneComponent.K2_SetWorldLocation` (`self.StaticMesh`) (`self.InitialLocation`) false false))

(event `self.ReceiveBeginPlay`
  (set `self.InitialLocation` (`SceneComponent.K2_GetComponentLocation` (`self.StaticMesh`))))

(fn `KeepVelocity`
  (params (DeltaTime :type "Float (double-precision)"))
  (bind _minredirectioninterval (`self.MinRedirectionInterval`))
  (if (`self.bIsInRound`)
    (`PrimitiveComponent.SetPhysicsLinearVelocity` (`self.StaticMesh`) (`KismetMathLibrary.MakeVector` (.x (* (`.Y` (`KismetMathLibrary.GetAxes` (`SceneComponent.K2_GetComponentRotation` (`self.StaticMesh`)))) (* (`self.MovementSpeed`) -1.0))) (.y (* (`.Y` (`KismetMathLibrary.GetAxes` (`SceneComponent.K2_GetComponentRotation` (`self.StaticMesh`)))) (* (`self.MovementSpeed`) -1.0))) -100.0) false "None")
    (bind _output_get (set `self.TimeToNextRedirection` (- (`self.TimeToNextRedirection`) DeltaTime)))
    (if (`self.bHitSpawner`)
      (set `self.bHitSpawner` false)
      (else
        (`/Engine/EditorBlueprintResources/StandardMacros.CompareFloat` _output_get
          (:`==`
            _)
          (:`<`
            _))
        (`SceneComponent.K2_SetWorldRotation` (`self.StaticMesh`) (`KismetMathLibrary.MakeRotator` 0.0 0.0 (* (`KismetMathLibrary.RandomFloat`) 360.0)) false false)))
    (set `self.TimeToNextRedirection` (+ (* (`KismetMathLibrary.RandomFloat`) (- (`self.MaxRedirectionInterval`) _minredirectioninterval)) _minredirectioninterval))))

(fn `LookAtCenterOfMap`
  (bind _staticmesh (`self.StaticMesh`))
  (`SceneComponent.K2_SetWorldRotation` _staticmesh (`KismetMathLibrary.MakeRotator` 0.0 0.0 (+ (.yaw (`KismetMathLibrary.FindLookAtRotation` (`SceneComponent.K2_GetComponentLocation` _staticmesh) (`KismetMathLibrary.MakeVector` 0.0))) 90.0)) false false))

(fn `ResetState`)

(fn `UserConstructionScript`)