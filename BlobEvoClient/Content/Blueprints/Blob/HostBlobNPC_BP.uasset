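; HostBlobNPC_BP is the host-side NPC blob, a child Blueprint that wanders by changing direction at random intervals during a round.
; Tick runs a countdown that, on expiry, sets a random rotation and reports the mesh's world transform through BlobDirectionComm.
; The timer re-rolls between min and max intervals at round start and after each turn.
; A spawner hit re-rolls it without turning.
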(event `self.ReceiveBeginPlay`
  (`parent.ReceiveBeginPlay`))

(event `self.ReceiveTick`
  (params (DeltaSeconds :type "Float (single-precision)"))
  (`parent.ReceiveTick` DeltaSeconds)
  (if (`self.bIsInRound`)
    (`self.ManageRotation` DeltaSeconds)))

(fn `BeginRound`
  (`parent.BeginRound`)
  (`self.RandomizeTimeToRedirection`))

(fn `CheckHit`
  (params (Other :type "Object Object Reference"))
  (`parent.CheckHit` Other))

(fn `LookAtCenterOfMap`
  (`parent.LookAtCenterOfMap`))

(fn `ManageRotation`
  (params (DeltaTIme :type "Float (double-precision)"))
  (bind _output_get (set `self.TimeToNextRedirection` (- (`self.TimeToNextRedirection`) DeltaTIme)))
  (if (`self.bHitSpawner`)
    (set `self.bHitSpawner` false)
    (else
      (`/Engine/EditorBlueprintResources/StandardMacros.CompareFloat` _output_get
        (:`==`
          _)
        (:`<`
          _))
      (`self.SetRotation` (* (`KismetMathLibrary.RandomFloat`) 360.0))
      (`BlobDirectionCommunicator.ReportNewBlobDirection` (`self.BlobDirectionComm`) (`self.ID`) (`SceneComponent.K2_GetComponentToWorld` (`self.StaticMesh`)))
      (set `self.bIsLookingAtCenterOfMap` false)))
  (`self.RandomizeTimeToRedirection`))

(fn `RandomizeTimeToRedirection`
  (bind _minredirectioninterval (`self.MinRedirectionInterval`))
  (set `self.TimeToNextRedirection` (+ (* (`KismetMathLibrary.RandomFloat`) (- (`self.MaxRedirectionInterval`) _minredirectioninterval)) _minredirectioninterval)))

(fn `UserConstructionScript`
  (`parent.UserConstructionScript`))