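; Client-side blob NPC actor that turns its mesh to match directions received for it.
; Each tick, after the parent logic, it asks BlobDirectionComm whether a new direction exists for its ID.
; When one is found, it sets the static mesh's world yaw to that value, applied directly without interpolation.
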(event `self.ReceiveBeginPlay`
  (`parent.ReceiveBeginPlay`))

(event `self.ReceiveTick`
  (params (DeltaSeconds :type "Float (single-precision)"))
  (`parent.ReceiveTick` DeltaSeconds)
  (`self.ListenForRotation`))

(fn `ListenForRotation`
  (bind (_outdirection _returnvalue) (`BlobDirectionCommunicator.CheckForNewBlobDirection` (`self.BlobDirectionComm`) (`self.ID`)))
  (if _returnvalue
    (`SceneComponent.K2_SetWorldRotation` (`self.StaticMesh`) (`KismetMathLibrary.MakeRotator` 0.0 0.0 (`KismetMathLibrary.Conv_IntToDouble` _outdirection)) false false)))

(fn `UserConstructionScript`
  (`parent.UserConstructionScript`))