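; Player pawn that owns a population of blobs and drives it through rounds of survival and reproduction.
; On BeginPlay it requests a starting batch from BlobSpawner_BP and stores it in the Blobs array.
; BeginRound and EndRound are relayed to each blob, with EndRound first running AssessBlobs.
; AssessBlobs destroys blobs failing ShouldLive and spawns offspring for survivors, modifying Blobs while looping over it.
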(event `self.ReceiveTick`
  (params (DeltaSeconds :type "Float (single-precision)")))

(event `self.ReceiveBeginPlay`
  (`self.SpawnAndSaveBlobs` (`self.BlobsPerPlayer`)))

(event `BeginRound`
  (for _array_element (`self.Blobs`)
    (bind _asblob_npc_bp (cast `/Game/Blueprints/BlobNPC_BP` _array_element))
    (`/Game/Blueprints/BlobNPC_BP.BeginRound` _asblob_npc_bp)))

(event `EndRound`
  (`self.AssessBlobs`)
  (for _array_element (`self.Blobs`)
    (bind _asblob_npc_bp (cast `/Game/Blueprints/BlobNPC_BP` _array_element))
    (`/Game/Blueprints/BlobNPC_BP.EndRound` _asblob_npc_bp)))

(fn `AssessBlobs`
  (bind _blobs (`self.Blobs`))
  (for _array_element _blobs
    (bind _asblob (cast `Blob` _array_element))
    (bind _returnvalue (`Blob.ShouldLive` _asblob))
    (if _returnvalue
      (bind _returnvalue_2 (`Blob.GetNumberOfNewBlobs` _asblob))
      (if true
        (`self.SpawnAndSaveBlobs` _returnvalue_2))
      (else
        (`KismetArrayLibrary.Array_RemoveItem` _blobs _asblob)
        (`self.K2_DestroyActor` _asblob)))))

(fn `SpawnAndSaveBlobs`
  (params (BlobsToSpawn :type Integer))
  (bind _returnvalue (`GameplayStatics.GetActorOfClass` "/Game/Blueprints/BlobSpawner_BP.BlobSpawner_BP_C"))
  (bind _returnvalue_2 (`Spawner.SpawnByCount` _returnvalue BlobsToSpawn))
  (for _array_element _returnvalue_2
    (bind _asblob (cast `Blob` _array_element))
    (`KismetArrayLibrary.Array_Add` (`self.Blobs`) _asblob)))

(fn `UserConstructionScript`)