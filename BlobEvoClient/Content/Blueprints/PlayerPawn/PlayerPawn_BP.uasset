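; Player pawn Blueprint that reports its movement and manages a collection of Blob NPCs through rounds.
; On BeginPlay it caches the PlayerServerCommunicator actor found in the world.
; Each tick, if the mesh's physics velocity is non-zero, it sends its ID and world location to that communicator.
; BeginRound and EndRound events are forwarded to every blob in its Blobs array, whose count it also exposes.
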(event `self.ReceiveTick`
  (params (DeltaSeconds :type "Float (single-precision)"))
  (`self.ReportLocation`))

(event `self.ReceiveBeginPlay`
  (bind _returnvalue (`GameplayStatics.GetActorOfClass` "/Script/BlobEvo.PlayerServerCommunicator"))
  (set `self.PlayerServerComm` _returnvalue))

(event `BeginRound`
  (for _array_element (`self.Blobs`)
    (bind _asblob_npc_bp (cast `/Game/Blueprints/Blob/BlobNPC_BP` _array_element))
    (`/Game/Blueprints/Blob/BlobNPC_BP.BeginRound` _asblob_npc_bp)))

(event `EndRound`
  (for _array_element (`self.Blobs`)
    (bind _asblob_npc_bp (cast `/Game/Blueprints/Blob/BlobNPC_BP` _array_element))
    (`/Game/Blueprints/Blob/BlobNPC_BP.EndRound` _asblob_npc_bp)))

(fn `GetNumberOfBlobs`
  (returns (NumberOfBlobs :type Integer))
  (return (`KismetArrayLibrary.Array_Length` (`self.Blobs`))))

(fn `ReportLocation`
  (locals (MovementVector :type "Vector Structure"))
  (bind _returnvalue (`PrimitiveComponent.GetPhysicsLinearVelocity` (`self.MeshComponent`) "None"))
  (if (not (== _returnvalue (0.0 0.0 0.0)))
    (`PlayerServerCommunicator.ReportNewLocation` (`self.PlayerServerComm`) (`self.ID`) (`SceneComponent.K2_GetComponentLocation` (`self.MeshComponent`)))))

(fn `UserConstructionScript`)